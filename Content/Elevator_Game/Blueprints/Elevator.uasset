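; Elevator actor whose two sliding doors are driven by custom Open_Door and Close_Door events.
; Each event runs its own timeline, with separate Left and Right tracks setting the relative Y location of the LeftDoor and RightDoor components.
; Opening plays the Open timeline forward, while closing plays the separate Close timeline in reverse from its end.
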(event `Open_Door`
  (bind (_direction _left _right) (`Timeline|Open`)
    (:`Update`
      (`SceneComponent.K2_SetRelativeLocation` (`self.LeftDoor`) (`KismetMathLibrary.MakeVector` 0.0 _left) false false)
      (`SceneComponent.K2_SetRelativeLocation` (`self.RightDoor`) (`KismetMathLibrary.MakeVector` 0.0 _right) false false))))

(event `Close_Door`
  (bind (_direction _left _right) (`Timeline|Close` :!via `ReverseFromEnd`)
    (:`Update`
      (`SceneComponent.K2_SetRelativeLocation` (`self.LeftDoor`) (`KismetMathLibrary.MakeVector` 0.0 _left) false false)
      (`SceneComponent.K2_SetRelativeLocation` (`self.RightDoor`) (`KismetMathLibrary.MakeVector` 0.0 _right) false false))))

(fn `UserConstructionScript`)